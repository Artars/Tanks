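; GM_Basic is a game mode that registers tanks by team and assigns players to their crew roles.
; SetTank stores each tank in a map, and SetDriver fills a team's Driver, Shooter or Captain slot only if that team has a tank and the slot is free.
; A successful assignment attaches the crew member to the tank, creates a new player, increments the player count and returns success.
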(fn `Set Driver`
  (params (Team :type Integer) (`Driver Ref` :type "/Game/Blueprints/BP_Crew Object Reference") (Role :type "/Game/Blueprints/ENUM_Crew_Class Enum" :default "NewEnumerator0"))
  (returns (Sucess :type Boolean))
  (locals (Work :type Boolean) (Tank :type "/Game/Blueprints/BP_Tank Object Reference"))
  (bind _tanks (`self.Tanks`))
  (bind _numplayers (`self.NumPlayers`))
  (bind _shooters (`self.Shooters`))
  (bind _work (`local.Work`))
  (bind _captains (`self.Captains`))
  (bind _output_get (set `local.Work` (`BlueprintMapLibrary.Map_Contains` _tanks Team)))
  (if _output_get
    (set `local.Tank` (`BlueprintMapLibrary.Map_Find` _tanks Team))
    (switch `/Game/Blueprints/ENUM_Crew_Class` Role
      (:`NewEnumerator0`
        (bind _output_get_2 (set `local.Work` (not (`BlueprintMapLibrary.Map_Contains` (`self.Drivers`) Team))))
        (if _output_get_2
          (`BlueprintMapLibrary.Map_Add` (`self.Drivers`) Team `Driver Ref`)
          (`/Game/Blueprints/BP_Tank.AddDriver` (`local.Tank`) `Driver Ref`)))
      (:`NewEnumerator1`
        (bind _output_get_3 (set `local.Work` (not (`BlueprintMapLibrary.Map_Contains` _shooters Team))))
        (if _output_get_3
          (`BlueprintMapLibrary.Map_Add` _shooters Team `Driver Ref`)
          (`/Game/Blueprints/BP_Tank.AddShooter` (`local.Tank`) `Driver Ref`)))
      (:`NewEnumerator2`
        (bind _output_get_4 (set `local.Work` (not (`BlueprintMapLibrary.Map_Contains` _captains Team))))
        (if _output_get_4
          (`BlueprintMapLibrary.Map_Add` _captains Team `Driver Ref`)
          (`/Game/Blueprints/BP_Tank.AddCaptain` (`local.Tank`) `Driver Ref`)))))
  (if _work
    (`GameplayStatics.CreatePlayer` _numplayers)
    (`/Engine/EditorBlueprintResources/StandardMacros.IncrementInt` _numplayers
      (:`  `
        _)))
  (return _work))

(fn `Set Tank`
  (params (TankRef :type "/Game/Blueprints/BP_Tank Object Reference") (Player :type Integer))
  (`BlueprintMapLibrary.Map_Add` (`self.Tanks`) Player TankRef))

(fn `UserConstructionScript`)