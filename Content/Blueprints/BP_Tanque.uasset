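; BP_Tanque is a tank Blueprint that turns using separate left and right thrust values.
; Tick passes both thrusts to MoveTank, which applies world yaw from right minus left, scaled by RotationVelocity and delta time, without sweep.
; MoveTank only rotates the actor and applies no translation.
; Debug strings print the thrust values and delta time every frame.
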(event `self.ReceiveTick`
  (params (DeltaSeconds :type "Float (single-precision)"))
  (bind _returnvalue (`self.GetInputAxisValue`))
  (bind _returnvalue_2 (`self.GetInputAxisValue`))
  (`self.MoveTank` _returnvalue_2 _returnvalue)
  (`KismetSystemLibrary.PrintString` (`KismetStringLibrary.Concat_StrStr` (`KismetStringLibrary.Conv_DoubleToString` _returnvalue_2) "," (`KismetStringLibrary.Conv_DoubleToString` _returnvalue))))

(fn `MoveTank`
  (params (LeftAxis :type "Float (double-precision)") (RightAxis :type "Float (double-precision)"))
  (bind _returnvalue (`GameplayStatics.GetWorldDeltaSeconds`))
  (`KismetSystemLibrary.PrintString` (`KismetStringLibrary.Conv_DoubleToString` _returnvalue))
  (`self.K2_AddActorWorldRotation` (`KismetMathLibrary.MakeRotator` 0.0 0.0 (* (- RightAxis LeftAxis) _returnvalue (`self.RotationVelocity`)))))

(fn `UserConstructionScript`)