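; BP_Captain is a player-controlled captain actor that turns its view in response to camera input.
; The Camera Horizontal and Camera Vertical axis events drive yaw and pitch, each scaled by its own speed variable and frame delta time.
; Both rotate the whole actor in local space with no pitch clamp, so combined turns can accumulate roll.
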(event `InputAxis|Camera Horizontal`
  (params (AxisValue :type "Float (single-precision)"))
  (`self.K2_AddActorLocalRotation` (`KismetMathLibrary.MakeRotator` 0.0 0.0 (* AxisValue (`self.HorizontalRotationSpeed`) (`GameplayStatics.GetWorldDeltaSeconds`)))))

(event `InputAxis|Camera Vertical`
  (params (AxisValue :type "Float (single-precision)"))
  (`self.K2_AddActorLocalRotation` (`KismetMathLibrary.MakeRotator` 0.0 (* AxisValue (`self.VerticalRotationSpeed`) (`GameplayStatics.GetWorldDeltaSeconds`)))))

(fn `UserConstructionScript`)