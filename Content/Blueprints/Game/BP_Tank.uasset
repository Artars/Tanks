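; Player-driven, networked tank pawn with thrust and health HUDs and a spawned cannon on a rotation pivot.
; Per-track thrust axes, zeroed when that side's ground traces miss, drive capped physics velocity and hull yaw, with the pivot counter-rotated to hold aim.
; Authority pushes hull and turret transforms to remotes each tick without interpolation.
; Authority also applies enemy bullet damage, reporting death to GM_Base, which handles respawn on destruction.
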(event `Assing local Controller`
  (bind _returnvalue (`GameplayStatics.GetPlayerController` 0))
  ;[1 1 1] Attach HUD
  (bind _returnvalue_2 (`|CreateWidget` "/Game/HUD/Gameplay/HUD_Thrust.HUD_Thrust_C" _returnvalue self))
  (bind _output_get (set `self.ThrustHUD` _returnvalue_2))
  (`UserWidget.AddToViewport` _output_get 0)
  (bind _returnvalue_3 (`|CreateWidget` "/Game/HUD/Gameplay/HUD_Health.HUD_Health_C" _returnvalue self))
  (bind _output_get_2 (set `self.HUDHealthRef` _returnvalue_3))
  (`UserWidget.AddToViewport` _output_get_2 1))

(event `self.ReceiveBeginPlay`
  ;[1 1 1] Spawn Turret and set Default Position
  (`self.SpawnTurret`))

(event `self.ReceivePossessed`
  (params (NewController :type "Controller Object Reference"))
  (bind _asplayer_controller (cast `PlayerController` NewController :!pure true))
  ;[1 1 1] Attach HUD
  (if (`Controller.IsLocalController` NewController)
    (bind _returnvalue (`|CreateWidget` "/Game/HUD/Gameplay/HUD_Thrust.HUD_Thrust_C" _asplayer_controller self))
    (bind _output_get (set `self.ThrustHUD` _returnvalue))
    (`UserWidget.AddToViewport` _output_get 0)
    (bind _returnvalue_2 (`|CreateWidget` "/Game/HUD/Gameplay/HUD_Health.HUD_Health_C" _asplayer_controller self))
    (bind _output_get_2 (set `self.HUDHealthRef` _returnvalue_2))
    (`UserWidget.AddToViewport` _output_get_2 1)
    (else
      (`self.Assing local Controller`))))

(event `self.ReceiveTick`
  (params (DeltaSeconds :type "Float (single-precision)"))
  ;[1 1 1] Updates tank position
  (`self.MoveTank` (select `bool` (`self.LeftOnTheGround`) :`true` (`self.LeftThrust`)) (select `bool` (`self.RightOnTheGround`) :`true` (`self.RightThrust`)))
  (set `self.ShootCounter` (- (`self.ShootCounter`) (`GameplayStatics.GetWorldDeltaSeconds`)))
  (`/Engine/EditorBlueprintResources/ActorMacros.Switch Has Authority`
    (:`Authority`
      (`self.Client Smooth Transform` (`self.GetTransform`) (`SceneComponent.RelativeRotation` (`self.RotationAxis`)))
      (`self.CheckGround`))))

(event `MoveTank`
  (params (LeftAxis :type "Float (double-precision)") (RightAxis :type "Float (double-precision)"))
  (bind _returnvalue (* LeftAxis RightAxis))
  (bind _returnvalue_2 (`KismetMathLibrary.FMin` LeftAxis RightAxis))
  ;[0.0918 1 0] Movment Management
  ;;[1 1 1] Mov a tank, give each imput axis
  ;;;[0.5204 1 0.9801] Rotate tank and cannon
  (`self.ServerApplyRotation` (- LeftAxis RightAxis))
  ;;;[0.9922 1 0.3191] Move the tank
  (if (and (not (`KismetMathLibrary.NearlyEqual_FloatFloat` _returnvalue 0.0 0.001)) (> _returnvalue 0.0))
    (`self.ServerApplyVelocity` (select `bool` (> _returnvalue_2 0.0) :`false` (* (`KismetMathLibrary.FMax` LeftAxis RightAxis) (`self.BackWardVelocity`) 1.0) :`true` (* _returnvalue_2 (`self.ForwardVelocity`) 1.0)) (`SceneComponent.GetForwardVector` (`self.Arrow`)))))

(event `IncrementRightThrust`
  (params (Axis :type "Float (double-precision)"))
  ;[0.0918 1 0] Movment Management
  ;;[1 1 1] Increase the right thrust value
  (set `self.RightThrust` (`KismetMathLibrary.FClamp` (+ (* Axis (`GameplayStatics.GetWorldDeltaSeconds`) (`self.ThrustSpeed`)) (`self.RightThrust`)) -1.0)))

(event `IncrementLeftThrust`
  (params (Axis :type "Float (double-precision)"))
  ;[0.0918 1 0] Movment Management
  ;;[1 1 1] Increase the left thrust variable
  (set `self.LeftThrust` (`KismetMathLibrary.FClamp` (+ (* Axis (`GameplayStatics.GetWorldDeltaSeconds`) (`self.ThrustSpeed`)) (`self.LeftThrust`)) -1.0)))

(event `Break`
  (params (Axis :type "Float (double-precision)"))
  (bind _returnvalue (* (`GameplayStatics.GetWorldDeltaSeconds`) Axis 5.0))
  ;[0.0918 1 0] Movment Management
  ;;[1 1 1] Reduce thrust when press brake
  (set `self.RightThrust` (`KismetMathLibrary.Lerp` (`self.RightThrust`) 0.0 _returnvalue))
  (set `self.LeftThrust` (`KismetMathLibrary.Lerp` (`self.LeftThrust`) 0.0 _returnvalue)))

(event `ServerApplyRotation`
  (params (Scale :type "Float (double-precision)"))
  (bind _returnvalue (`SceneComponent.GetUpVector` (`self.Arrow`)))
  (bind _returnvalue_2 (* Scale (`self.RotationVelocity`) (`GameplayStatics.GetWorldDeltaSeconds`)))
  ;[1 1 1] Server events
  (`self.K2_AddActorWorldRotation` (`KismetMathLibrary.RotatorFromAxisAndAngle` _returnvalue _returnvalue_2))
  (`SceneComponent.K2_AddLocalRotation` (`self.RotationAxis`) (`KismetMathLibrary.RotatorFromAxisAndAngle` _returnvalue (* _returnvalue_2 -1.0)) false false))

(event `ServerApplyVelocity`
  (params (Scale :type "Float (double-precision)") (Direction :type "Vector Structure"))
  (bind _returnvalue (`SceneComponent.GetForwardVector` (`self.Arrow`)))
  ;[1 1 1] Server events
  (`PrimitiveComponent.SetPhysicsLinearVelocity` (`self.Body`) (* _returnvalue (* (`self.Aceleration`) 1.0 1.0)) true "None")
  (bind _returnvalue_2 (`PrimitiveComponent.GetPhysicsLinearVelocity` (`self.Body`) "None"))
  (if (> (`KismetMathLibrary.Abs` (`KismetMathLibrary.Dot_VectorVector` _returnvalue _returnvalue_2)) (`KismetMathLibrary.Abs` Scale))
    (`PrimitiveComponent.SetPhysicsLinearVelocity` (`self.Body`) (* (`KismetMathLibrary.Normal` _returnvalue_2) Scale) false "None")))

(event `InputAxis|Break`
  (params (AxisValue :type "Float (single-precision)"))
  ;[1 0 0.09896] Input
  (`self.Break` AxisValue))

(event `InputAxis|Right Thrust`
  (params (AxisValue :type "Float (single-precision)"))
  ;[1 0 0.09896] Input
  (`self.IncrementRightThrust` AxisValue))

(event `InputAxis|Left Thrust`
  (params (AxisValue :type "Float (single-precision)"))
  ;[1 0 0.09896] Input
  (`self.IncrementLeftThrust` AxisValue))

(event `Client Smooth Transform`
  (params (Transform :type "Transform Structure") (TurretRot :type "Rotator Structure"))
  ;[1 1 1] Server events
  (`/Engine/EditorBlueprintResources/ActorMacros.Switch Has Authority`
    (:`Remote`
      (`self.K2_SetActorTransform` Transform)
      (`SceneComponent.K2_SetRelativeRotation` (`self.RotationAxis`) TurretRot false false))))

(event `SpawnTurret`
  ;[1 1 1] Server events
  (`/Engine/EditorBlueprintResources/StandardMacros.IsValid` (`self.Cannon`)
    (:`Is Not Valid`
      (bind _returnvalue (`|SpawnActorFromClass` "/Game/Blueprints/Game/BP_Cannon.BP_Cannon_C" (`SceneComponent.K2_GetComponentToWorld` (`self.RotationAxis`)) "Undefined" "OverrideRootScale" null self null))
      (bind _output_get (set `self.Cannon` _returnvalue))
      (`self.K2_AttachToComponent` _output_get (`self.RotationAxis`) "None" "KeepWorld" "KeepWorld" "KeepWorld" true)
      (bind _returnvalue_2 (`PoseableMeshComponent.GetBoneRotationByName` (`/Game/Blueprints/Game/BP_Cannon.Mesh` _output_get) "Cannon" "ComponentSpace"))
      (set `self.InitialBoneRotation` _returnvalue_2))))

(event `self.ReceiveHit`
  (params (MyComp :type "PrimitiveComponent Object Reference") (Other :type "Actor Object Reference") (OtherComp :type "PrimitiveComponent Object Reference") (bSelfMoved :type Boolean) (HitLocation :type "Vector Structure") (HitNormal :type "Vector Structure") (NormalImpulse :type "Vector Structure") (Hit :type "HitResult Structure (by ref)"))
  ;[1 1 1] On collision / Teeats damage
  (`/Engine/EditorBlueprintResources/ActorMacros.Switch Has Authority`
    (:`Authority`
      (bind _asbp_bullet (cast `/Game/Blueprints/Game/BP_Bullet` Other))
      (`self.Treat Bullet Collsion` _asbp_bullet))))

(event `Treat Bullet Collsion`
  (params (Bullet :type "/Game/Blueprints/Game/BP_Bullet Object Reference"))
  (if (!= (`/Game/Blueprints/Game/BP_Bullet.Player` Bullet) (`self.Team`))
    (bind _output_get (set `self.Health` (- (`self.Health`) (`/Game/Blueprints/Game/BP_Bullet.Damage` Bullet))))
    (`/Game/Blueprints/Game/BP_Bullet.CallDestroyAll` Bullet)
    (if (<= _output_get 0.0)
      (bind _asgm_base (cast `/Game/Blueprints/Game/GM_Base` (`GameplayStatics.GetGameMode`)))
      (`/Game/Blueprints/Game/GM_Base.TankDied` _asgm_base (`self.Team`)))))

(event `Respawn`
  ;[1 1 1] Treats Respawn
  (set `self.Health` (`self.MaxHealth`)))

(event `CheckGround`
  (bind _hitcheckfr (`self.HitCheckFR`))
  (bind _hitcheckbr (`self.HitCheckBR`))
  (bind _hitcheckfl (`self.HitCheckFL`))
  (bind _hitcheckbl (`self.HitCheckBL`))
  (bind _returnvalue (`SceneComponent.K2_GetComponentLocation` _hitcheckbl))
  (bind _returnvalue_2 (`SceneComponent.K2_GetComponentLocation` _hitcheckfr))
  (bind _returnvalue_3 (`SceneComponent.K2_GetComponentLocation` _hitcheckbr))
  (bind _returnvalue_4 (`SceneComponent.K2_GetComponentLocation` _hitcheckfl))
  (bind (_outhit _returnvalue_5) (`KismetSystemLibrary.LineTraceSingle` _returnvalue_3 (+ _returnvalue_3 (* (`SceneComponent.GetForwardVector` _hitcheckbr) (`self.DistanceToCheckGround`))) "TraceTypeQuery1"))
  (bind (_outhit_2 _returnvalue_6) (`KismetSystemLibrary.LineTraceSingle` _returnvalue_2 (+ _returnvalue_2 (* (`SceneComponent.GetForwardVector` _hitcheckfr) (`self.DistanceToCheckGround`))) "TraceTypeQuery1"))
  (set `self.RightOnTheGround` (or _returnvalue_5 _returnvalue_6))
  (bind (_outhit_3 _returnvalue_7) (`KismetSystemLibrary.LineTraceSingle` _returnvalue_4 (+ _returnvalue_4 (* (`SceneComponent.GetForwardVector` _hitcheckfl) (`self.DistanceToCheckGround`))) "TraceTypeQuery1"))
  (bind (_outhit_4 _returnvalue_8) (`KismetSystemLibrary.LineTraceSingle` _returnvalue (+ _returnvalue (* (`SceneComponent.GetForwardVector` _hitcheckbl) (`self.DistanceToCheckGround`))) "TraceTypeQuery1"))
  (set `self.LeftOnTheGround` (or _returnvalue_7 _returnvalue_8)))

(event `self.ReceiveDestroyed`
  (`self.ForceRespawn`))

(event `ForceRespawn`
  (bind _asgm_base (cast `/Game/Blueprints/Game/GM_Base` (`GameplayStatics.GetGameMode`)))
  (`/Game/Blueprints/Game/GM_Base.RespawnTank` _asgm_base (`self.Team`)))

(fn `UserConstructionScript`)