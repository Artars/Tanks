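; BP_Cannon is a possessable tank cannon that turns, elevates and fires BP_Bullet on a cooldown, spawning an attached captain and creating a health HUD.
; Input sends only direction changes and stops through Server-to-Client event pairs with current angles to resync, while Tick integrates motion locally.
; Yaw rotates the actor and counter-rotates the captain's camera mount; elevation poses the clamped "Cannon" bone.
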(event `Assing local Controller`
  (bind _returnvalue (`|CreateWidget` "/Game/HUD/HUD_Health.HUD_Health_C" (`GameplayStatics.GetPlayerController` 0) (`self.Tank`)))
  (bind _output_get (set `self.HUDHealthRef` _returnvalue))
  (`UserWidget.AddToViewport` _output_get 1))

(event `self.ReceivePossessed`
  (params (NewController :type "Controller Object Reference"))
  (if (`Controller.IsLocalController` NewController)
    (bind _returnvalue (`|CreateWidget` "/Game/HUD/HUD_Health.HUD_Health_C" (cast `PlayerController` NewController :!pure true) (`self.Tank`)))
    (bind _output_get (set `self.HUDHealthRef` _returnvalue))
    (`UserWidget.AddToViewport` _output_get 1)
    (else
      (`self.Assing local Controller`))))

(event `AddCaptain`
  (bind _captainspawnposition (`self.CaptainSpawnPosition`))
  (bind _returnvalue (`|SpawnActorFromClass` "/Game/Blueprints/Game/BP_Captain.BP_Captain_C" (`SceneComponent.K2_GetComponentToWorld` _captainspawnposition) "Undefined" "OverrideRootScale" null (`self.Tank`) null))
  (bind _output_get (set `/Game/Blueprints/Game/BP_Tank.Captain` _returnvalue (`self.Tank`)))
  (`self.K2_AttachToComponent` _output_get _captainspawnposition "None" "KeepWorld" "KeepWorld" "KeepWorld" true))

(event `UpdateRotation`
  (bind _captaincameralocation (`self.CaptainCameraLocation`))
  (bind _turningdirection (`self.TurningDirection`))
  (bind (_relativerotation_roll _relativerotation_pitch _relativerotation_yaw) (`KismetMathLibrary.BreakRotator` (`SceneComponent.RelativeRotation` _captaincameralocation)))
  (bind _returnvalue (+ (* (`KismetMathLibrary.Conv_IntToDouble` _turningdirection) (`GameplayStatics.GetWorldDeltaSeconds`) (`self.CannonSpeed`)) (.yaw (struct))))
  (if (!= _turningdirection 0)
    (`self.K2_AddActorLocalRotation` (`KismetMathLibrary.MakeRotator` 0.0 0.0 _returnvalue))
    (`SceneComponent.K2_SetRelativeRotation` _captaincameralocation (`KismetMathLibrary.MakeRotator` _relativerotation_roll _relativerotation_pitch (+ (* -1 _returnvalue) _relativerotation_yaw)) false false)))

(event `self.ReceiveBeginPlay`
  (bind _returnvalue (`PoseableMeshComponent.GetBoneRotationByName` (`self.Mesh`) "Cannon" "ComponentSpace"))
  (set `self.InitialBoneRotation` _returnvalue)
  (`self.AddCaptain`))

(event `self.ReceiveTick`
  (params (DeltaSeconds :type "Float (single-precision)"))
  (set `self.ShootCounter` (- (`self.ShootCounter`) (`GameplayStatics.GetWorldDeltaSeconds`)))
  (`self.UpdateRotation`)
  (`self.UpdateNivel`))

(event `UpdateNivel`
  (bind _niveldirection (`self.NivelDirection`))
  (if (!= _niveldirection 0)
    (bind _output_get (set `self.CannonNivel` (`KismetMathLibrary.FClamp` (- (`self.CannonNivel`) (* (`self.ElevationSpeed`) (`KismetMathLibrary.Conv_IntToDouble` _niveldirection) (`GameplayStatics.GetWorldDeltaSeconds`))) (`self.CannonMaxNivel`) 0.0)))
    (`PoseableMeshComponent.SetBoneRotationByName` (`self.Mesh`) "Cannon" (`KismetMathLibrary.ComposeRotators` (`KismetMathLibrary.MakeRotator` _output_get) (`self.InitialBoneRotation`)) "ComponentSpace")))

(event `TurnEvent`
  (params (Axis :type "Float (double-precision)"))
  (bind _captaincameralocation (`self.CaptainCameraLocation`))
  (bind (_relativerotation_roll _relativerotation_pitch _relativerotation_yaw) (`KismetMathLibrary.BreakRotator` (`SceneComponent.RelativeRotation` _captaincameralocation)))
  (bind _returnvalue (+ (* Axis (`GameplayStatics.GetWorldDeltaSeconds`) (`self.CannonSpeed`)) (.yaw (struct))))
  ;[1 0.8653 0] Shooting related events
  ;;[1 1 1] Turn cannon given an axis input
  (`self.K2_AddActorLocalRotation` (`KismetMathLibrary.MakeRotator` 0.0 0.0 _returnvalue))
  (`SceneComponent.K2_SetRelativeRotation` _captaincameralocation (`KismetMathLibrary.MakeRotator` _relativerotation_roll _relativerotation_pitch (+ (* -1 _returnvalue) _relativerotation_yaw)) false false))

(event `ServerChangeDirection`
  (params (Direction :type Integer) (Rotation :type "Rotator Structure"))
  (`self.ClientChangeDirection` Direction Rotation))

(event `ClientChangeDirection`
  (params (Direction :type Integer) (Rotation :type "Rotator Structure"))
  (set `self.TurningDirection` Direction)
  (`SceneComponent.K2_SetRelativeRotation` (`self.DefaultSceneRoot`) Rotation false false))

(event `ServerStopRotating`
  (params (Rotation :type "Rotator Structure"))
  (`self.ClientStopRotating` Rotation))

(event `NivelCannon`
  (params (Axis :type "Float (double-precision)"))
  ;[1 0.8653 0] Shooting related events
  ;;[1 1 1] Ajust cannon nivel
  (bind _output_get (set `self.CannonNivel` (`KismetMathLibrary.FClamp` (- (`self.CannonNivel`) (* (`self.ElevationSpeed`) Axis (`GameplayStatics.GetWorldDeltaSeconds`))) (`self.CannonMaxNivel`) 0.0)))
  (`PoseableMeshComponent.SetBoneRotationByName` (`self.Mesh`) "Cannon" (`KismetMathLibrary.ComposeRotators` (`KismetMathLibrary.MakeRotator` _output_get) (`self.InitialBoneRotation`)) "ComponentSpace"))

(event `ClientStopRotating`
  (params (Rotation :type "Rotator Structure"))
  (set `self.TurningDirection` 0)
  (`SceneComponent.K2_SetRelativeRotation` (`self.DefaultSceneRoot`) Rotation false false))

(event `ServerChangeNivel`
  (params (Direction :type Integer) (CurrentNivel :type "Float (double-precision)"))
  (`self.ClientChangeNivel` Direction CurrentNivel))

(event `Shoot`
  (params (Transform :type "Transform Structure") (Speed :type "Float (double-precision)"))
  (`self.SpawnBullet` Transform Speed))

(event `SpawnBullet`
  (params (Transform :type "Transform Structure") (Speed :type "Float (double-precision)"))
  ;[1 0.8653 0] Shooting related events
  ;;[1 1 1] Shoot a bullet
  (bind _returnvalue (`|SpawnActorFromClass` "/Game/Blueprints/Game/BP_Bullet.BP_Bullet_C" Transform "Undefined" "OverrideRootScale" null null))
  (set `ProjectileMovementComponent.MaxSpeed` Speed (`/Game/Blueprints/Game/BP_Bullet.ProjectileMovement` _returnvalue)))

(event `ClientChangeNivel`
  (params (Direction :type Integer) (`Current Nivel` :type "Float (double-precision)"))
  (set `self.NivelDirection` Direction)
  (bind _output_get (set `self.CannonNivel` `Current Nivel`))
  (`PoseableMeshComponent.SetBoneRotationByName` (`self.Mesh`) "Cannon" (`KismetMathLibrary.ComposeRotators` (`KismetMathLibrary.MakeRotator` _output_get) (`self.InitialBoneRotation`)) "ComponentSpace"))

(event `ServerStopNivel`
  (params (CurrentNivel :type "Float (double-precision)"))
  (`self.ClientStopNivel` CurrentNivel))

(event `InputAxis|Turn Cannon`
  (params (AxisValue :type "Float (single-precision)"))
  (bind _returnvalue (* (`KismetMathLibrary.Round` AxisValue) (`self.TurningDirection`)))
  (bind _relativerotation (`SceneComponent.RelativeRotation` (`self.DefaultSceneRoot`)))
  (if (and (== (`self.TurningDirection`) 0) (not (`KismetMathLibrary.NearlyEqual_FloatFloat` AxisValue 0.0 0.1)))
    (bind _output_get (set `self.TurningDirection` (`KismetMathLibrary.Round` AxisValue) :!label _label))
    (`self.ServerChangeDirection` _output_get _relativerotation)
    (elif (< _returnvalue 0)
      (goto _label)
      (elif (== _returnvalue 0)
        (set `self.TurningDirection` 0)
        (`self.ServerStopRotating` _relativerotation)))))

(event `ClientStopNivel`
  (params (CurrentNivel :type "Float (double-precision)"))
  (set `self.NivelDirection` 0)
  (bind _output_get (set `self.CannonNivel` CurrentNivel))
  (`PoseableMeshComponent.SetBoneRotationByName` (`self.Mesh`) "Cannon" (`KismetMathLibrary.ComposeRotators` (`KismetMathLibrary.MakeRotator` _output_get) (`self.InitialBoneRotation`)) "ComponentSpace"))

(event `InputAxis|Cannon Incl`
  (params (AxisValue :type "Float (single-precision)"))
  (bind _cannonnivel (`self.CannonNivel`))
  (bind _returnvalue (* (`KismetMathLibrary.Round` AxisValue) (`self.NivelDirection`)))
  (if (and (== (`self.NivelDirection`) 0) (not (`KismetMathLibrary.NearlyEqual_FloatFloat` AxisValue 0.0 0.1)))
    (bind _output_get (set `self.NivelDirection` (`KismetMathLibrary.Round` AxisValue) :!label _label_2))
    (`self.ServerChangeNivel` _output_get _cannonnivel)
    (elif (< _returnvalue 0)
      (goto _label_2)
      (elif (== _returnvalue 0)
        (set `self.NivelDirection` 0)
        (`self.ServerStopNivel` _cannonnivel)))))

(event `InputAction|Fire`
  (params (Key :type "Key Structure"))
  (:`Pressed`
    (if (<= (`self.ShootCounter`) 0.0)
      (`self.Shoot` (`KismetMathLibrary.MakeTransform` (.location (`SceneComponent.K2_GetComponentToWorld` (`self.SpawnPoint`))) (.rotation (`SceneComponent.K2_GetComponentToWorld` (`self.SpawnPoint`)))) (`self.ProjectileSpeed`))
      (set `self.ShootCounter` (`self.ShootInterval`)))))

(fn `TurnCannon`)

(fn `UserConstructionScript`)