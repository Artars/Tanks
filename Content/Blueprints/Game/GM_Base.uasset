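; Game mode for a multiplayer team tank game, spawning one tank per team at random spawn points.
; Swapped-in controllers request team 1, possessing its tank, cannon or captain by role if that slot is free.
; Controllers arriving before their tank exists wait in a pending list processed after spawning.
; Tank deaths are counted per team and trigger respawn and teleport; logout calls the game instance's session-destroy handler.
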(event `self.K2_OnSwapPlayerControllers`
  (params (OldPC :type "PlayerController Object Reference") (NewPC :type "PlayerController Object Reference"))
  ;[1 1 1] Add entering players
  (`KismetArrayLibrary.Array_Add` (`self.AllPlayerControllers`) NewPC)
  (bind _asgameplay_pc (cast `/Game/Blueprints/Gameplay/GameplayPC` NewPC))
  (`self.RespawnPlayer` NewPC (`.MyPlayerRole_10_63F1AC1248B92C5FDC101F89BBB40BED` (break `/Game/Blueprints/AllLeves/PlayerInfo` (`/Game/Blueprints/Gameplay/GameplayPC.PlayerSettings` _asgameplay_pc))) 1))

(event `self.ReceiveBeginPlay`
  ;[1 1 1] Get number of teams and call tank spawn
  (bind _asgame_info_instance (cast `/Game/Blueprints/AllLeves/GameInfoInstance` (`GameplayStatics.GetGameInstance`)))
  (set `self.NumTeams` (`/Game/Blueprints/AllLeves/GameInfoInstance.NumTeams` _asgame_info_instance))
  (bind _outactors (`GameplayStatics.GetAllActorsOfClass` "/Game/Blueprints/Game/BP_Spawn_Tank.BP_Spawn_Tank_C"))
  (bind _output_get (set `self.TankSpawns` _outactors))
  (set `self.RemainingSpawns` _output_get)
  (`self.SpawnTanks`))

(event `SpawnTanks`
  ;[1 1 1] Spawn tanks according to number of teams
  (for _index (range 1 (+ (`self.NumTeams`) 1))
    (bind _transform (`self.GetTankSpawn`))
    (bind _returnvalue (`|SpawnActorFromClass` "/Game/Blueprints/Game/BP_Tank.BP_Tank_C" _transform "Undefined" "OverrideRootScale" null _index null))
    (`BlueprintMapLibrary.Map_Add` (`self.Tanks`) _index _returnvalue)
    (`BlueprintMapLibrary.Map_Add` (`self.Deaths`) _index))
  (for _array_element (`self.PendingControllers`)
    (bind _asgameplay_pc (cast `/Game/Blueprints/Gameplay/GameplayPC` _array_element))
    (bind (_myplayername _myplayerimage _myplayerrole _myplayerteam) (break `/Game/Blueprints/AllLeves/PlayerInfo` (`/Game/Blueprints/Gameplay/GameplayPC.PlayerSettings` _asgameplay_pc)))
    (`self.Assign Player` _array_element _myplayerrole _myplayerteam)
    (`KismetArrayLibrary.Array_RemoveItem` (`self.PendingControllers`) _array_element)))

(event `RespawnTank`
  (params (Team :type Integer))
  (bind _value (`BlueprintMapLibrary.Map_Find` (`self.Tanks`) Team))
  ;[1 1 1] Respawn a given tank
  (`/Game/Blueprints/Game/BP_Tank.Respawn` _value)
  (bind _transform (`self.GetTankSpawn`))
  (`self.K2_SetActorTransform` _value _transform false true))

(event `self.K2_OnLogout`
  (params (ExitingController :type "Controller Object Reference"))
  ;[1 1 1] Event on logout / Destroy session caller
  (bind _asgameplay_pc (cast `/Game/Blueprints/Gameplay/GameplayPC` ExitingController))
  (`/Game/Blueprints/AllLeves/GameInfoInstance.DestroySessionCaller` (cast `/Game/Blueprints/AllLeves/GameInfoInstance` (`GameplayStatics.GetGameInstance`) :!pure true) _asgameplay_pc))

(event `RespawnPlayer`
  (params (PlayerController :type "PlayerController Object Reference") (Class :type "/Game/Blueprints/Game/ENUM_Crew_Class Enum" :default "NewEnumerator0") (Team :type Integer))
  ;[1 1 1] Assign Player to each tank
  (`KismetArrayLibrary.Array_Add` (`self.SpawnedPlayers`) PlayerController)
  (if (`.ReturnValue` (`BlueprintMapLibrary.Map_Find` (`self.Tanks`) Team))
    (`self.Assign Player` PlayerController Class Team)
    (else
      (`KismetArrayLibrary.Array_Add` (`self.PendingControllers`) PlayerController))))

(event `TankDied`
  (params (Team :type Integer))
  (bind _deaths (`self.Deaths`))
  ;[1 1 1] DIEDED
  (if (not (`.ReturnValue` (`BlueprintMapLibrary.Map_Find` _deaths Team)))
    (`BlueprintMapLibrary.Map_Add` _deaths Team))
  (`/Engine/EditorBlueprintResources/StandardMacros.IncrementInt` (`BlueprintMapLibrary.Map_Find` _deaths Team)
    (:`  `
      (`self.RespawnTank` Team))))

(fn `Assign Player`
  (params (Controller :type "PlayerController Object Reference") (Class :type "/Game/Blueprints/Game/ENUM_Crew_Class Enum" :default "NewEnumerator0") (Team :type Integer))
  (returns (Sucess :type Boolean))
  (locals (HasSucedded :type Boolean))
  (bind (_value _returnvalue) (`BlueprintMapLibrary.Map_Find` (`self.Tanks`) Team))
  (bind _cannon (`/Game/Blueprints/Game/BP_Tank.Cannon` _value))
  (if _returnvalue
    (if (`|EnumEquality` Class "NewEnumerator0")
      (if (not (`.ReturnValue` (`BlueprintMapLibrary.Map_Find` (`self.Drivers`) Team)))
        (`Controller.Possess` Controller _value)
        (`self.SetOwner` _value Controller)
        (`BlueprintMapLibrary.Map_Add` (`self.Drivers`) Team Controller)
        (set `local.HasSucedded` true))
      (elif (`|EnumEquality` Class "NewEnumerator1")
        (if (not (`.ReturnValue` (`BlueprintMapLibrary.Map_Find` (`self.Shooters`) Team)))
          (`Controller.Possess` Controller _cannon)
          (`self.SetOwner` Controller _cannon)
          (`BlueprintMapLibrary.Map_Add` (`self.Shooters`) Team Controller)
          (set `local.HasSucedded` true))
        (elif (`|EnumEquality` Class "NewEnumerator2")
          (if (not (`.ReturnValue` (`BlueprintMapLibrary.Map_Find` (`self.Captains`) Team)))
            (`BlueprintMapLibrary.Map_Add` (`self.Captains`) Team Controller)
            (`Controller.Possess` Controller (`/Game/Blueprints/Game/BP_Tank.Captain` _value))
            (set `local.HasSucedded` true))))))
  (return (`local.HasSucedded`)))

(fn `GetTankSpawn`
  (returns (Transform :type "Transform Structure"))
  (locals (ToReturn :type "Transform Structure") (Ref :type "/Game/Blueprints/Game/BP_Spawn_Tank Object Reference"))
  (bind _remainingspawns (`self.RemainingSpawns`))
  (if (> (`KismetArrayLibrary.Array_Length` _remainingspawns) 0)
    (set `self.RemainingSpawns` (`self.TankSpawns`)))
  (bind _output_get (set `local.Ref` (`|GetArrayItem` _remainingspawns (`KismetMathLibrary.RandomIntegerInRange` 0 (`KismetArrayLibrary.Array_LastIndex` _remainingspawns)))))
  (set `local.ToReturn` (`self.GetTransform` _output_get))
  (`KismetArrayLibrary.Array_RemoveItem` (`self.RemainingSpawns`) _output_get)
  (return (`local.ToReturn`)))

(fn `Set Tank`
  (params (TankRef :type "/Game/Blueprints/Game/BP_Tank Object Reference") (Player :type Integer))
  (`BlueprintMapLibrary.Map_Add` (`self.Tanks`) Player TankRef))

(fn `UserConstructionScript`)