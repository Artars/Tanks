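; BP_Crew represents one tank crew member, turning player input into tank commands according to its role: Driver, Shooter or Captain.
; BeginPlay derives the role from NumberRole, and input events require a valid Tank and matching role.
; Only the Driver's left and right thrust reach the Tank; brake, cannon and fire inputs are empty stubs.
; Assign creates the Driver's thrust HUD, but its only call here is disconnected.
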(event `Assign`
  (switch `/Game/Blueprints/Game/ENUM_Crew_Class` (`self.Class`)
    (:`NewEnumerator0`
      (bind _returnvalue (`|CreateWidget` "/Game/HUD/Gameplay/HUD_Thrust.HUD_Thrust_C" (`GameplayStatics.GetPlayerController` 0) null))
      (bind _output_get (set `self.HUDRef` _returnvalue))
      (`UserWidget.AddToViewport` _output_get 0)
      (`/Game/HUD/Gameplay/HUD_Thrust.SetController` (`self.HUDRef`) (`self.Tank`)))))

(event `self.ReceiveBeginPlay`
  (set `self.Class` (select `int` (`self.NumberRole`) :`0` "NewEnumerator3" :`1` "NewEnumerator0" :`2` "NewEnumerator1" :`3` "NewEnumerator2" :!type "/Game/Blueprints/Game/ENUM_Crew_Class Enum"))
  (cast `/Game/Blueprints/Game/GM_Base` (`GameplayStatics.GetGameMode`)))

(event `InputAxis|Right Thrust`
  (params (AxisValue :type "Float (single-precision)"))
  ;[0 0.3671 1] Driver Function
  (if (and (`KismetSystemLibrary.IsValid` (`self.Tank`)) (`|EnumEquality` (`self.Class`) "NewEnumerator0"))
    (`/Game/Blueprints/Game/BP_Tank.IncrementRightThrust` (`self.Tank`) AxisValue)))

(event `InputAxis|Left Thrust`
  (params (AxisValue :type "Float (single-precision)"))
  ;[0 0.3671 1] Driver Function
  (if (and (`KismetSystemLibrary.IsValid` (`self.Tank`)) (`|EnumEquality` (`self.Class`) "NewEnumerator0"))
    (`/Game/Blueprints/Game/BP_Tank.IncrementLeftThrust` (`self.Tank`) AxisValue)))

(event `InputAxis|Break`
  (params (AxisValue :type "Float (single-precision)"))
  ;[0 0.3671 1] Driver Function
  (if (and (`KismetSystemLibrary.IsValid` (`self.Tank`)) (`|EnumEquality` (`self.Class`) "NewEnumerator0"))
    _))

(event `InputAxis|Turn Cannon`
  (params (AxisValue :type "Float (single-precision)"))
  ;[1 0 0.02864] Shooter functions
  (if (and (`KismetSystemLibrary.IsValid` (`self.Tank`)) (`|EnumEquality` (`self.Class`) "NewEnumerator1"))
    _))

(event `InputAxis|Cannon Incl`
  (params (AxisValue :type "Float (single-precision)"))
  ;[1 0 0.02864] Shooter functions
  (if (and (`KismetSystemLibrary.IsValid` (`self.Tank`)) (`|EnumEquality` (`self.Class`) "NewEnumerator1"))
    _))

(event `InputAction|Fire`
  (params (Key :type "Key Structure"))
  ;[1 0 0.02864] Shooter functions
  (:`Pressed`
    (if (and (`KismetSystemLibrary.IsValid` (`self.Tank`)) (`|EnumEquality` (`self.Class`) "NewEnumerator1"))
      _)))

(fn `UserConstructionScript`)