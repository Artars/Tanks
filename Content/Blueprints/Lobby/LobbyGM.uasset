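; Lobby game mode that manages joining, leaving, kicking, character availability and map launch for a multiplayer match.
; On login it pulls server settings from GameInfoInstance, initializes each LobbyPC and possesses a crew pawn at a random PlayerStart.
; EveryoneUpdate rebuilds player info, pushes it to all controllers and sets CanWeStart from role and team choices.
; Host setting changes propagate to every controller, and launch server-travels to the selected arena.
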(event `YouHaveBeenKicked`
  (params (PlayerID :type Integer))
  ;[1 1 1] Kick a selected player from the lobby
  (`/Game/Blueprints/Lobby/LobbyPC.Kicked` (cast `/Game/Blueprints/Lobby/LobbyPC` (`|GetArrayItem` (`self.AllPlayerControllers`) PlayerID) :!pure true)))

(event `self.K2_PostLogin`
  (params (NewPlayer :type "PlayerController Object Reference"))
  ;[1 1 1] Initial Setup called when players login and call setup on lobby menu and spawn players
  (`/Engine/EditorBlueprintResources/ActorMacros.Switch Has Authority`
    (:`Authority`
      (`KismetArrayLibrary.Array_Add` (`self.AllPlayerControllers`) NewPlayer)
      (bind _outactors (`GameplayStatics.GetAllActorsOfClass` "/Script/Engine.PlayerStart"))
      (set `self.SpawnPoints` _outactors)
      (bind _asgame_info_instance (cast `/Game/Blueprints/AllLeves/GameInfoInstance` (`GameplayStatics.GetGameInstance`)))
      (set `self.ServerName` (`/Game/Blueprints/AllLeves/GameInfoInstance.ServerName` _asgame_info_instance))
      (set `self.MaxPlayers` (`/Game/Blueprints/AllLeves/GameInfoInstance.MaxPlayers` _asgame_info_instance))
      (set `self.NumTeams` (`/Game/Blueprints/AllLeves/GameInfoInstance.NumTeams` _asgame_info_instance))
      (bind _aslobby_pc (cast `/Game/Blueprints/Lobby/LobbyPC` NewPlayer))
      (`/Game/Blueprints/Lobby/LobbyPC.InitialSetup` _aslobby_pc)
      (`/Game/Blueprints/Lobby/LobbyPC.SetupLobbyMenu` _aslobby_pc (`self.ServerName`) (`self.MaxPlayers`) (`self.NumTeams`))
      (`/Game/Blueprints/Lobby/LobbyPC.UpdateLobbySettings` _aslobby_pc (`self.GM_MapImage`) (`self.GM_MapName`) (`self.GM_MapTime`))
      (`self.RespawnPlayer` NewPlayer)
      (`/Engine/EditorBlueprintResources/StandardMacros.DoOnce` false
        (:`Completed`
          (`self.CreateAvailableArray` (`self.MaxPlayers`)))))))

(event `self.K2_OnLogout`
  (params (ExitingController :type "Controller Object Reference"))
  (bind _allplayercontrollers (`self.AllPlayerControllers`))
  ;[1 1 1] Event OnLogout -  Removes Player controller and connected player Info / Resets Avalable characters
  (for (_array_element _array_index) _allplayercontrollers
    (if (== _array_element ExitingController)
      (break)))
  (bind _aslobby_pc (cast `/Game/Blueprints/Lobby/LobbyPC` (`|GetArrayItem` _allplayercontrollers _array_index)))
  (`KismetArrayLibrary.Array_Set` (`self.AvailableCharacters`) (`/Game/Blueprints/Lobby/LobbyPC.SelectedCharacter` _aslobby_pc))
  (`KismetArrayLibrary.Array_Remove` (`self.AllPlayerControllers`) _array_index)
  (`KismetArrayLibrary.Array_Remove` (`self.ConnectedPlayers`) _array_index)
  (`self.EveryoneUpdate`))

(event `RespawnPlayer`
  (params (PlayerController :type "PlayerController Object Reference"))
  (bind _returnvalue (`Controller.K2_GetPawn` PlayerController))
  (bind _spawnpoints (`self.SpawnPoints`))
  ;[1 1 1] Respawn player at base character in lobby / Everyine update the lobby
  (`/Engine/EditorBlueprintResources/StandardMacros.IsValid` _returnvalue
    (:`Is Valid`
      (`self.K2_DestroyActor` _returnvalue))
    (:`Is Not Valid`
      _))
  (bind _returnvalue_2 (`|SpawnActorFromClass` "/Game/Blueprints/Game/BP_Crew.BP_Crew_C" (`self.GetTransform` (`|GetArrayItem` _spawnpoints (`KismetMathLibrary.RandomIntegerInRange` 0 (- (`KismetArrayLibrary.Array_Length` _spawnpoints) 1)))) "Undefined" "OverrideRootScale" null 0 0 null))
  (`Controller.Possess` PlayerController _returnvalue_2)
  (`self.EveryoneUpdate`))

(event `ServerUpdateGameSettings`
  (params (MapImage :type "Texture2D Object Reference") (MapName :type Text) (MapTime :type Text) (MapID :type Integer))
  ;[1 1 1] Server has made changes / Tell Cliants to update lobby information
  (set `self.GM_MapImage` MapImage)
  (set `self.GM_MapName` MapName)
  (set `self.GM_MapTime` MapTime)
  (set `self.GM_MapID` MapID)
  (for _array_element (`self.AllPlayerControllers`)
    (bind _aslobby_pc (cast `/Game/Blueprints/Lobby/LobbyPC` _array_element))
    (`/Game/Blueprints/Lobby/LobbyPC.UpdateLobbySettings` _aslobby_pc (`self.GM_MapImage`) (`self.GM_MapName`) (`self.GM_MapTime`))))

(event `AddToKickList`
  ;[1 1 1] Add a player to the ick list if game settings window is open
  (bind _aslobby_pc (cast `/Game/Blueprints/Lobby/LobbyPC` (`GameplayStatics.GetPlayerController` 0)))
  (bind _lobbymenuwb (`/Game/Blueprints/Lobby/LobbyPC.LobbyMenuWB` _aslobby_pc))
  (`/Engine/EditorBlueprintResources/StandardMacros.IsValid` _lobbymenuwb
    (:`Is Valid`
      (bind _gamesettings (`/Game/HUD/Lobby/LobbyMenu.GameSettings` _lobbymenuwb))
      (if (`Widget.IsVisible` _gamesettings)
        (`/Game/HUD/Lobby/GameSettings.FillPlayersWindow` _gamesettings)))))

(event `EveryoneUpdate`
  (bind _allplayercontrollers (`self.AllPlayerControllers`))
  ;[1 1 1] Updates on connected ´players lobby information call
  (bind _output_get (set `self.CurrentPlayers` (`KismetArrayLibrary.Array_Length` (`self.AllPlayerControllers`))))
  (if (> _output_get 0)
    (`KismetArrayLibrary.Array_Clear` (`self.ConnectedPlayers`))
    (for _array_element _allplayercontrollers
      (bind _aslobby_pc (cast `/Game/Blueprints/Lobby/LobbyPC` _array_element))
      (`KismetArrayLibrary.Array_Add` (`self.ConnectedPlayers`) (`/Game/Blueprints/Lobby/LobbyPC.PlayerSettings` _aslobby_pc))
      (`/Game/Blueprints/Lobby/LobbyPC.UpdateNumberOfPlayers` _aslobby_pc (`self.CurrentPlayers`) (`self.MaxPlayers`)))
    (for _array_element_2 _allplayercontrollers
      (bind _aslobby_pc_2 (cast `/Game/Blueprints/Lobby/LobbyPC` _array_element_2))
      (`/Game/Blueprints/Lobby/LobbyPC.AddPlayerInfo` _aslobby_pc_2 (`self.ConnectedPlayers`))
      (`/Game/Blueprints/Lobby/LobbyPC.UpdateAvailableCharacters` _aslobby_pc_2 (`self.AvailableCharacters`))
      (`self.AddToKickList`))
    (for _array_element_3 (`self.ConnectedPlayers`) :!label _label
      (bind (_myplayername _myplayerimage _myplayerrole _myplayerteam) (break `/Game/Blueprints/AllLeves/PlayerInfo` _array_element_3))
      (if (or (`|EnumEquality` _myplayerrole "NewEnumerator3") (== _myplayerteam 0))
        (set `self.CanWeStart?` false)
        (`self.CannotStartGame`)
        (else
          (set `self.CanWeStart?` true))))))

(event `LaunchTheGame`
  (bind _returnvalue (`GameplayStatics.GetPlayerController` 0))
  ;[1 1 1] Lauch game base on map selections from game settings
  (switch `int` (`self.GM_MapID`)
    (:`0`
      (`KismetSystemLibrary.ExecuteConsoleCommand` "servertravel /Game/Maps/Arenas/Arena01" _returnvalue))
    (:`1`
      (`KismetSystemLibrary.ExecuteConsoleCommand` "servertravel /Game/Maps/Arenas/Arena02" _returnvalue))))

(event `SwapCharacter`
  (params (PlayerController :type "PlayerController Object Reference") (CrewRole :type "/Game/Blueprints/Game/ENUM_Crew_Class Enum" :default "NewEnumerator0") (PlayerTeam :type Integer) (ChangedStatus :type Boolean))
  (bind _returnvalue (`Controller.K2_GetPawn` PlayerController))
  (bind _spawnpoints (`self.SpawnPoints`))
  ;[1 1 1] Swap the current character to the selected character
  (if (not ChangedStatus)
    (`/Engine/EditorBlueprintResources/StandardMacros.IsValid` _returnvalue
      (:`Is Valid`
        (`self.K2_DestroyActor` _returnvalue))
      (:`Is Not Valid`
        _))
    (bind _returnvalue_2 (`|SpawnActorFromClass` "/Game/Blueprints/Lobby/LobbyObserver.LobbyObserver_C" (`self.GetTransform` (`|GetArrayItem` _spawnpoints (`KismetMathLibrary.RandomIntegerInRange` 0 (- (`KismetArrayLibrary.Array_Length` _spawnpoints) 1)))) "Undefined" "OverrideRootScale" null null))
    (`Controller.Possess` PlayerController _returnvalue_2)))

(event `CannotStartGame`
  ;[1 1 1] Updates on connected ´players lobby information call
  (goto _label :!via `Break`))

(fn `CreateAvailableArray`
  (params (NumPlayers :type Integer))
  (`KismetArrayLibrary.Array_Clear` (`self.AvailableCharacters`))
  (for _ (range 1 (+ NumPlayers 1))
    (`KismetArrayLibrary.Array_Add` (`self.AvailableCharacters`))))

(fn `UserConstructionScript`)