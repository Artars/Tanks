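; Player tank crewed by a driver, shooter and captain, who attach at camera points; it registers with GM_Basic and spawns an attached BP_Cannon.
; Tick drives differential steering from two thrust values, counter-rotating the turret axis to keep aim independent of the hull.
; Cannon yaw counter-rotates the captain camera, elevation rotates a mesh bone, and firing spawns BP_Bullet on a cooldown.
; Direct input bindings are debug-only, gated by flags.
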(event `self.ReceiveBeginPlay`
  (bind _asgm_basic (cast `/Game/Blueprints/GM_Basic` (`GameplayStatics.GetGameMode`)))
  (`/Game/Blueprints/GM_Basic.Set Tank` _asgm_basic self 0)
  (bind _returnvalue (`|SpawnActorFromClass` "/Game/Blueprints/BP_Cannon.BP_Cannon_C" (`SceneComponent.K2_GetComponentToWorld` (`self.RotationAxis`)) "Undefined" "OverrideRootScale" null null))
  (bind _output_get (set `self.Cannon` _returnvalue))
  (`self.K2_AttachToComponent` _output_get (`self.RotationAxis`) "None" "KeepWorld" "KeepWorld" "KeepWorld" true)
  (bind _returnvalue_2 (`PoseableMeshComponent.GetBoneRotationByName` (`/Game/Blueprints/BP_Cannon.Mesh` _output_get) "Cannon" "ComponentSpace"))
  (set `self.InitialBoneRotation` _returnvalue_2))

(event `self.ReceiveTick`
  (params (DeltaSeconds :type "Float (single-precision)"))
  (`self.MoveTank` (`self.LeftThrust`) (`self.RightThrust`))
  (set `self.ShootCounter` (- (`self.ShootCounter`) (`GameplayStatics.GetWorldDeltaSeconds`))))

(event `InputAxis|Right Thrust`
  (params (AxisValue :type "Float (single-precision)"))
  ;[1 0 0.09896] DEBUG
  (if (`self.DebbugDriving`)
    (`self.IncrementRightThrust` AxisValue)
    (`PrimitiveComponent.SetOwnerNoSee` (`self.Body`) false)))

(event `InputAxis|Left Thrust`
  (params (AxisValue :type "Float (single-precision)"))
  ;[1 0 0.09896] DEBUG
  (if (`self.DebbugDriving`)
    (`self.IncrementLeftThrust` AxisValue)))

(event `InputAxis|Turn Cannon`
  (params (AxisValue :type "Float (single-precision)"))
  ;[1 0 0.09896] DEBUG
  (if (`self.DebbugShooting`)
    (`self.TurnCannon` AxisValue)))

(event `InputAxis|Cannon Incl`
  (params (AxisValue :type "Float (single-precision)"))
  ;[1 0 0.09896] DEBUG
  (if (`self.DebbugShooting`)
    (`self.NivelCannon` AxisValue)))

(event `InputAction|Fire`
  (params (Key :type "Key Structure"))
  ;[1 0 0.09896] DEBUG
  (:`Pressed`
    (if (`self.DebbugShooting`)
      (`self.Shoot`))))

(fn `AddCaptain`
  (params (NewCaptain :type "/Game/Blueprints/BP_Crew Object Reference"))
  (bind _captaincameralocation (`/Game/Blueprints/BP_Cannon.CaptainCameraLocation` (`self.Cannon`)))
  (bind _output_get (set `self.Captain` NewCaptain))
  (`self.K2_SetActorTransform` _output_get (`SceneComponent.K2_GetComponentToWorld` _captaincameralocation) false false)
  (`self.K2_AttachToComponent` _output_get _captaincameralocation "None" "KeepWorld" "KeepWorld" "KeepWorld" true)
  (set `/Game/Blueprints/BP_Crew.Tank` self (`self.Captain`)))

(fn `AddDriver`
  (params (NewDriver :type "/Game/Blueprints/BP_Crew Object Reference"))
  (bind _output_get (set `self.Driver` NewDriver))
  (`self.K2_SetActorTransform` _output_get (`SceneComponent.K2_GetComponentToWorld` (`self.DriverCameraPoint`)) false false)
  (`self.K2_AttachToActor` _output_get self "None" "KeepWorld" "KeepWorld" "KeepWorld" true)
  (set `/Game/Blueprints/BP_Crew.Tank` self _output_get)
  (`self.SetOwner` _output_get))

(fn `AddShooter`
  (params (NewShooter :type "/Game/Blueprints/BP_Crew Object Reference"))
  (bind _shooter (`self.Shooter`))
  (bind _shootercameralocation (`/Game/Blueprints/BP_Cannon.ShooterCameraLocation` (`self.Cannon`)))
  (bind _output_get (set `self.Shooter` NewShooter))
  (`self.K2_SetActorTransform` _output_get (`SceneComponent.K2_GetComponentToWorld` _shootercameralocation) false false)
  (`self.K2_AttachToComponent` _output_get _shootercameralocation "None" "KeepWorld" "KeepWorld" "KeepWorld" true)
  (set `/Game/Blueprints/BP_Crew.Tank` self _shooter)
  (`self.SetOwner` (`self.Cannon`) _shooter))

(fn `Break`
  (params (Axis :type "Float (double-precision)"))
  (bind _returnvalue (* (`GameplayStatics.GetWorldDeltaSeconds`) Axis 5.0))
  (set `self.RightThrust` (`KismetMathLibrary.Lerp` (`self.RightThrust`) 0.0 _returnvalue))
  (set `self.LeftThrust` (`KismetMathLibrary.Lerp` (`self.LeftThrust`) 0.0 _returnvalue)))

(fn `IncrementLeftThrust`
  (params (Axis :type "Float (double-precision)"))
  (set `self.LeftThrust` (`KismetMathLibrary.FClamp` (+ (* Axis (`GameplayStatics.GetWorldDeltaSeconds`) (`self.ThrustSpeed`)) (`self.LeftThrust`)) -1.0)))

(fn `IncrementRightThrust`
  (params (Axis :type "Float (double-precision)"))
  (set `self.RightThrust` (`KismetMathLibrary.FClamp` (+ (* Axis (`GameplayStatics.GetWorldDeltaSeconds`) (`self.ThrustSpeed`)) (`self.RightThrust`)) -1.0)))

(fn `MoveTank`
  (params (LeftAxis :type "Float (double-precision)" :default 0.0) (RightAxis :type "Float (double-precision)" :default 0.0))
  (bind _returnvalue (`GameplayStatics.GetWorldDeltaSeconds`))
  (bind _returnvalue_2 (* LeftAxis RightAxis))
  (bind _returnvalue_3 (`KismetMathLibrary.FMin` LeftAxis RightAxis))
  (bind _rotationaxis (`self.RotationAxis`))
  (bind _returnvalue_4 (`SceneComponent.GetForwardVector` (`self.Arrow`)))
  (bind _returnvalue_5 (* (- LeftAxis RightAxis) (`GameplayStatics.GetWorldDeltaSeconds`) (`self.RotationVelocity`)))
  (bind (_relativerotation_roll _relativerotation_pitch _relativerotation_yaw) (`KismetMathLibrary.BreakRotator` (`SceneComponent.RelativeRotation` _rotationaxis)))
  ;[0.5204 1 0.9801] Rotate tank and cannon
  (`self.K2_SetActorRotation` (`KismetMathLibrary.MakeRotator` (.roll (`self.K2_GetActorRotation`)) (.pitch (`self.K2_GetActorRotation`)) (+ _returnvalue_5 (.yaw (`self.K2_GetActorRotation`)))))
  (`SceneComponent.K2_SetRelativeRotation` _rotationaxis (`KismetMathLibrary.MakeRotator` _relativerotation_roll _relativerotation_pitch (+ (* -1 _returnvalue_5) _relativerotation_yaw)) false false)
  ;[0.9922 1 0.3191] Move the tank
  (if (and (!= _returnvalue_2 0.0) (> _returnvalue_2 0.0))
    (if (> _returnvalue_3 0.0)
      (`self.AddMovementInput` _returnvalue_4 (* _returnvalue_3 (`self.ForwardVelocity`) _returnvalue))
      (else
        (`self.AddMovementInput` _returnvalue_4 (* (`KismetMathLibrary.FMax` LeftAxis RightAxis) (`self.BackWardVelocity`) _returnvalue))))))

(fn `NivelCannon`
  (params (Axis :type "Float (double-precision)"))
  (bind _output_get (set `self.CannonNivel` (`KismetMathLibrary.FClamp` (- (`self.CannonNivel`) (* (`self.ElevationSpeed`) Axis (`GameplayStatics.GetWorldDeltaSeconds`))) (`self.CannonMaxNivel`) 0.0)))
  (`PoseableMeshComponent.SetBoneRotationByName` (`/Game/Blueprints/BP_Cannon.Mesh` (`self.Cannon`)) "Cannon" (`KismetMathLibrary.ComposeRotators` (`KismetMathLibrary.MakeRotator` _output_get) (`self.InitialBoneRotation`)) "ComponentSpace"))

(fn `Shoot`
  (if (<= (`self.ShootCounter`) 0.0)
    (`|SpawnActorFromClass` "/Game/Blueprints/BP_Bullet.BP_Bullet_C" (`KismetMathLibrary.MakeTransform` (.location (`SceneComponent.K2_GetComponentToWorld` (`/Game/Blueprints/BP_Cannon.SpawnPoint` (`self.Cannon`)))) (.rotation (`SceneComponent.K2_GetComponentToWorld` (`/Game/Blueprints/BP_Cannon.SpawnPoint` (`self.Cannon`))))) "Undefined" "OverrideRootScale" null null)
    (set `self.ShootCounter` (`self.ShootInterval`))))

(fn `TurnCannon`
  (params (Axis :type "Float (double-precision)" :default 0.0))
  (bind _captaincameralocation (`/Game/Blueprints/BP_Cannon.CaptainCameraLocation` (`self.Cannon`)))
  (bind _returnvalue (+ (* Axis (`GameplayStatics.GetWorldDeltaSeconds`) (`self.CannonSpeed`)) (.yaw (struct))))
  (bind (_relativerotation_roll _relativerotation_pitch _relativerotation_yaw) (`KismetMathLibrary.BreakRotator` (`SceneComponent.RelativeRotation` _captaincameralocation)))
  (`self.K2_AddActorLocalRotation` (`self.Cannon`) (`KismetMathLibrary.MakeRotator` 0.0 0.0 _returnvalue) false false)
  (`SceneComponent.K2_SetRelativeRotation` _captaincameralocation (`KismetMathLibrary.MakeRotator` _relativerotation_roll _relativerotation_pitch (+ (* -1 _returnvalue) _relativerotation_yaw)) false false))

(fn `UserConstructionScript`)