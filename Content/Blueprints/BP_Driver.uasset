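; BP_Driver is the player-side crew member of a tank, acting as either Driver or Shooter according to its Class.
; On BeginPlay it registers its team and role with GM_Basic, and for the Driver creates a thrust HUD bound to the Tank.
; Role-gated inputs forward to the referenced Tank: separate left/right thrust and brake for the Driver, cannon turning, inclination and firing for the Shooter.
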(event `self.ReceiveBeginPlay`
  (bind _asgm_basic (cast `/Game/Blueprints/GM_Basic` (`GameplayStatics.GetGameMode`)))
  (`/Game/Blueprints/GM_Basic.Set Driver` _asgm_basic (`self.Team`) self (`self.Class`))
  (switch `/Game/Blueprints/ENUM_Crew_Class` (`self.Class`)
    (:`NewEnumerator0`
      (bind _returnvalue (`|CreateWidget` "/Game/HUD/HUD_Thrust.HUD_Thrust_C"))
      (bind _output_get (set `self.HUDRef` _returnvalue))
      (`UserWidget.AddToViewport` _output_get 0)
      (`/Game/HUD/HUD_Thrust.SetController` (`self.HUDRef`) (`self.Tank`)))))

(event `InputAxis|Right Thrust`
  (params (AxisValue :type "Float (single-precision)"))
  ;[0 0.3671 1] Driver Function
  (if (and (`KismetSystemLibrary.IsValid` (`self.Tank`)) (`|EnumEquality` (`self.Class`) "NewEnumerator0"))
    (`/Game/Blueprints/BP_Tank.IncrementRightThrust` (`self.Tank`) AxisValue)))

(event `InputAxis|Left Thrust`
  (params (AxisValue :type "Float (single-precision)"))
  ;[0 0.3671 1] Driver Function
  (if (and (`KismetSystemLibrary.IsValid` (`self.Tank`)) (`|EnumEquality` (`self.Class`) "NewEnumerator0"))
    (`/Game/Blueprints/BP_Tank.IncrementLeftThrust` (`self.Tank`) AxisValue)))

(event `InputAxis|Break`
  (params (AxisValue :type "Float (single-precision)"))
  ;[0 0.3671 1] Driver Function
  (if (and (`KismetSystemLibrary.IsValid` (`self.Tank`)) (`|EnumEquality` (`self.Class`) "NewEnumerator0"))
    (`/Game/Blueprints/BP_Tank.Break` (`self.Tank`) AxisValue)))

(event `InputAxis|Turn Cannon`
  (params (AxisValue :type "Float (single-precision)"))
  ;[1 0 0.02864] Shooter functions
  (if (and (`KismetSystemLibrary.IsValid` (`self.Tank`)) (`|EnumEquality` (`self.Class`) "NewEnumerator1"))
    (`/Game/Blueprints/BP_Tank.TurnCannon` (`self.Tank`) AxisValue)))

(event `InputAxis|Cannon Incl`
  (params (AxisValue :type "Float (single-precision)"))
  ;[1 0 0.02864] Shooter functions
  (if (and (`KismetSystemLibrary.IsValid` (`self.Tank`)) (`|EnumEquality` (`self.Class`) "NewEnumerator1"))
    (`/Game/Blueprints/BP_Tank.NivelCannon` (`self.Tank`) AxisValue)))

(event `InputAction|Fire`
  (params (Key :type "Key Structure"))
  ;[1 0 0.02864] Shooter functions
  (:`Pressed`
    (if (and (`KismetSystemLibrary.IsValid` (`self.Tank`)) (`|EnumEquality` (`self.Class`) "NewEnumerator1"))
      (`/Game/Blueprints/BP_Tank.Shoot` (`self.Tank`)))))

(fn `UserConstructionScript`)